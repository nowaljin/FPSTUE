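; BP_AutoDoor is a two-panel sliding door that opens when the first-person player character enters its detection sphere and closes when they leave.
; On BeginPlay it caches each panel's closed position and derives open positions by offsetting them in opposite directions along relative X.
; A timeline lerps both panels between these positions, always restarting from its start or end, so an interrupted movement snaps before animating.
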(event OnComponentBeginOverlap(DetectionSphere)
  (params (OverlappedComponent :type Primitive%20Component%20Object%20Reference) (OtherActor :type Actor%20Object%20Reference) (OtherComp :type Primitive%20Component%20Object%20Reference) (OtherBodyIndex :type Integer) (bFromSweep :type Boolean) (SweepResult :type Hit%20Result%20Structure%20%28by%20ref%29))
  (if (.bSuccess (Utilities|Casting|CastToBP_FirstPersonCharacter OtherActor))
    (Variables|Default|SetIsPlayerNear true)
    (bind _dooranimation (Timeline|DoorTimeline PlayFromStart)
      (:Update
        (Transformation|SetRelativeLocation (Variables|Default|GetLeftDoor) (Math|Vector|Lerp(Vector) (Variables|Default|GetLeftDoorClosedPos) (Variables|Default|GetLeftDoorOpenPos) _dooranimation) false false)
        (Transformation|SetRelativeLocation (Variables|Default|GetRightDoor) (Math|Vector|Lerp(Vector) (Variables|Default|GetRightDoorClosedPos) (Variables|Default|GetRightDoorOpenPos) _dooranimation) false false)))))

(event OnComponentEndOverlap(DetectionSphere)
  (params (OverlappedComponent :type Primitive%20Component%20Object%20Reference) (OtherActor :type Actor%20Object%20Reference) (OtherComp :type Primitive%20Component%20Object%20Reference) (OtherBodyIndex :type Integer))
  (if (.bSuccess (Utilities|Casting|CastToBP_FirstPersonCharacter OtherActor))
    (Variables|Default|SetIsPlayerNear false)
    (bind _dooranimation (Timeline|DoorTimeline ReverseFromEnd)
      (:Update
        (Transformation|SetRelativeLocation (Variables|Default|GetLeftDoor) (Math|Vector|Lerp(Vector) (Variables|Default|GetLeftDoorClosedPos) (Variables|Default|GetLeftDoorOpenPos) _dooranimation) false false)
        (Transformation|SetRelativeLocation (Variables|Default|GetRightDoor) (Math|Vector|Lerp(Vector) (Variables|Default|GetRightDoorClosedPos) (Variables|Default|GetRightDoorOpenPos) _dooranimation) false false)))))

(event EventBeginPlay
  (Variables|Default|SetLeftDoorClosedPos (Variables|/Script/Engine.SceneComponent|GetRelativeLocation (Variables|Default|GetLeftDoor)))
  (Variables|Default|SetRightDoorClosedPos (Variables|/Script/Engine.SceneComponent|GetRelativeLocation (Variables|Default|GetRightDoor)))
  (Variables|Default|SetLeftDoorOpenPos (+ (Variables|Default|GetLeftDoorClosedPos) (Math|Vector|MakeVector (* (Variables|Default|GetDoorOpenDistance) (Math|Float|MakeLiteralFloat -1.0)) 0.0 0.0)))
  (Variables|Default|SetRightDoorOpenPos (+ (Variables|Default|GetRightDoorClosedPos) (Math|Vector|MakeVector (Variables|Default|GetDoorOpenDistance) 0.0 0.0))))

(event Collision|EventActorBeginOverlap
  (params (OtherActor :type Actor%20Object%20Reference)))

(event EventTick
  (params (DeltaSeconds :type Float%20%28single-precision%29)))

(fn ConstructionScript)